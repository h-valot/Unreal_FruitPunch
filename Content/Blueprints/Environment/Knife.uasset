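; Falling knife hazard that repeatedly strikes at random spots in an area and destroys any actor its Knife component hits.
; The TeleportKnife macro picks a random position and yaw at fixed height, then triggers a slow descent, fast drop and rise, separated by random pauses.
; A custom delayed-loop macro steps each movement with swept SetActorLocation calls, and the cycle restarts after the rise.
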(event OnComponentHit(Knife)
  (params (HitComponent :type Primitive%20Component%20Object%20Reference) (OtherActor :type Actor%20Object%20Reference) (OtherComp :type Primitive%20Component%20Object%20Reference) (NormalImpulse :type Vector :default "0, 0, 0") (Hit :type Hit%20Result%20Structure%20%28by%20ref%29))
  ;[1 1 1] kill on hit
  (Actor|DestroyActor OtherActor))

(event Custom|CustomEvent
  (bind _returnvalue (Transformation|GetActorLocation))
  (bind _returnvalue_2 (Transformation|GetActorLocation))
  (bind _returnvalue_3 (Transformation|GetActorLocation))
  (Utilities|Loop+Delay 0 75 0.01
    (:Loop%20Body
      (Transformation|SetActorLocation (Math|Vector|MakeVector (.x _returnvalue) (.y _returnvalue) (- (.z _returnvalue) 1e+01)) true false))
    (:Completed
      (Utilities|FlowControl|Delay (Math|Random|RandomFloatinRange 1.0 2.0))
      (Utilities|Loop+Delay 0 14 0.01
        (:Loop%20Body
          (Transformation|SetActorLocation (Math|Vector|MakeVector (.x _returnvalue_3) (.y _returnvalue_3) (- (.z _returnvalue_3) 35.0)) true false))
        (:Completed
          (Utilities|FlowControl|Delay (Math|Random|RandomFloatinRange 0.5 1.5))
          (Utilities|Loop+Delay 0 150 0.01
            (:Loop%20Body
              (Transformation|SetActorLocation (Math|Vector|MakeVector (.x _returnvalue_2) (.y _returnvalue_2) (+ (.z _returnvalue_2) 1e+01)) true false))
            (:Completed
              (Utilities|FlowControl|Delay (Math|Random|RandomFloatinRange 2.0 5.0))
              (Utilities|TeleportKnife))))))))

(event EventBeginPlay
  (Utilities|FlowControl|Delay (Math|Random|RandomFloatinRange 2.0 5.0))
  (Utilities|TeleportKnife))

(fn ConstructionScript)