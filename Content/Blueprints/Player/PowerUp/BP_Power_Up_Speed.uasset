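; Speed power-up pickup that boosts a BP_GenericCharacter on overlap.
; It destroys itself first, then calls ActivateSpeed on the character, raises MaxWalkSpeed and copies that value into CurrentSpeed.
; A Delay is meant to restore a lower speed after a few seconds, but it runs on the already destroyed pickup, so the reset is at risk of never firing.
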(event Collision|EventActorBeginOverlap
  (params (OtherActor :type Actor%20Object%20Reference))
  (bind _asbp_generic_character (Utilities|Casting|CastToBP_GenericCharacter OtherActor))
  (Actor|DestroyActor)
  (Default|ActivateSpeed _asbp_generic_character true)
  (bind _output_get (Variables|/Script/Engine.CharacterMovementComponent|SetMaxWalkSpeed (Variables|/Script/Engine.Character|GetCharacterMovement _asbp_generic_character) 1.2e+03))
  (Variables|/Game/Blueprints/Player/BP_GenericCharacter.BP_GenericCharacter_C|SetCurrentSpeed _asbp_generic_character _output_get)
  (Utilities|FlowControl|Delay 5.0)
  (bind _output_get_2 (Variables|/Script/Engine.CharacterMovementComponent|SetMaxWalkSpeed (Variables|/Script/Engine.Character|GetCharacterMovement _asbp_generic_character) 6e+02))
  (Variables|/Game/Blueprints/Player/BP_GenericCharacter.BP_GenericCharacter_C|SetCurrentSpeed _asbp_generic_character _output_get_2))

(fn ConstructionScript)