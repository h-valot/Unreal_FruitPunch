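; Game mode for local multiplayer that sets up one local player per PlayerStart, with a shared camera.
; On BeginPlay it finds the camera and game manager, creates players possessing input receiver pawns with menu input, removes CameraActors and starts both.
; SpawnPlayer, not called within this graph, adds game input, spawns and possesses a character at its receiver, then updates the camera's player list.
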(event EventBeginPlay
  (CallFunction|GetReferences)
  (CallFunction|SpawnInputReceivers)
  (CallFunction|RemoveUnusedCamera)
  (CallFunction|StartGame))

(fn ConstructionScript)

(fn GetReferences
  (CallFunction|GetPlayerStarts)
  (CallFunction|GetCamera)
  (CallFunction|GetScoreManager))

(fn GetPlayerStarts
  (bind _outactors (Actor|GetAllActorsOfClass "/Script/Engine.PlayerStart"))
  (Variables|Default|SetPlayerStarts _outactors))

(fn GetCamera
  (bind _outactors (Actor|GetAllActorsOfClass "/Game/Blueprints/Player/BP_Camera.BP_Camera_C"))
  (Variables|Default|SetCamera (Utilities|Array|Get(acopy) _outactors)))

(fn GetScoreManager
  (bind _outactors (Actor|GetAllActorsOfClass "/Game/Blueprints/Player/BP_GameManager.BP_GameManager_C"))
  (Variables|Default|SetGameManager (Utilities|Array|Get(acopy) _outactors)))

(fn SpawnInputReceivers
  (for (_array_element _array_index) (Variables|Default|GetPlayerStarts)
    (bind _output_get (LocalVariables|SetIndex _array_index))
    (bind _returnvalue (Class|GameplayStatics|CreatePlayer _output_get))
    (Utilities|Array|AddUnique (Variables|Default|GetPlayerControllers) _returnvalue)
    (Input|AddMappingContext (PlayerController|LocalPlayerSubsystems|GetEnhancedInputLocalPlayerSubsystem (CallFunction|GetCorrectController (LocalVariables|GetIndex))) "/Game/Inputs/IMC_Menu.IMC_Menu" 0 "(bIgnoreAllPressedKeysUntilRelease=True,bForceImmediately=False)")
    (bind _returnvalue_2 (Game|SpawnActorfromClass "/Game/Blueprints/Player/BP_InputReceiver.BP_InputReceiver_C" (Math|Transform|MakeTransform (.location (Transformation|GetActorTransform _array_element)) "0, 0, 0" "1.000000,1.000000,1.000000") "Undefined" "MultiplyWithRoot" 0 (LocalVariables|GetIndex) (.location (Transformation|GetActorTransform _array_element)) 0))
    (Utilities|Array|Add (Variables|Default|GetPlayerInputReceivers) _returnvalue_2)
    (Pawn|Possess (CallFunction|GetCorrectController (LocalVariables|GetIndex)) _returnvalue_2)))

(fn GetCorrectController
  (params (Index :type Integer))
  (if (> Index 0)
    (return (Utilities|Array|Get(acopy) (Variables|Default|GetPlayerControllers) Index))
    (else
      (return (Game|GetPlayerController 0)))))

(fn RemoveUnusedCamera
  (Actor|GetAllActorsOfClass "/Script/Engine.CameraActor")
  (for _array_element 0
    (Actor|DestroyActor _array_element)))

(fn StartGame
  (Default|StartGame (Variables|Default|GetCamera))
  (Default|GameStarted (Variables|Default|GetGameManager) (Variables|Default|GetPlayers)))

(fn SpawnPlayer
  (params (CurrentPlayerIndex :type Integer) (InputReceiver :type BP%20Input%20Receiver%20Object%20Reference))
  (bind _returnvalue (Game|GetPlayerController CurrentPlayerIndex))
  (bind _returnvalue_2 (Transformation|GetActorTransform InputReceiver))
  (Input|AddMappingContext (PlayerController|LocalPlayerSubsystems|GetEnhancedInputLocalPlayerSubsystem (CallFunction|GetCorrectController CurrentPlayerIndex)) "/Game/Inputs/IMC_Game.IMC_Game" 0 "(bIgnoreAllPressedKeysUntilRelease=True,bForceImmediately=False)")
  (bind _returnvalue_3 (Game|SpawnActorfromClass "/Game/Blueprints/Player/BP_GenericCharacter.BP_GenericCharacter_C" (Math|Transform|MakeTransform (.location _returnvalue_2) "0, 0, 0" "1.000000,1.000000,1.000000") "Undefined" "MultiplyWithRoot" 0 CurrentPlayerIndex (.location _returnvalue_2) 0))
  (Utilities|Array|Add (Variables|Default|GetPlayers) _returnvalue_3)
  (Pawn|Possess _returnvalue _returnvalue_3)
  (Game|Player|SetViewTargetwithBlend _returnvalue (Variables|Default|GetCamera) 0.0 "VTBlend_Linear" 0.0 false)
  (Default|UpdatePlayerList (Variables|Default|GetCamera) (Variables|Default|GetPlayers))
  (return false))