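; BP_Camera is a shared multiplayer camera that keeps a group of players framed once the game has started.
; Each tick it lerps a Sphere toward the average location of the player list, which is supplied through UpdatePlayerList.
; It then sets the spring arm length to the largest pairwise distance between players, clamped to a minimum and maximum, zooming out as they spread apart.
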(event EventTick
  (params (DeltaSeconds :type Float%20%28single-precision%29))
  (if (Variables|Default|GetbGameStarted)
    (CallFunction|CalculateCameraMovement)
    (CallFunction|CalculateCameraDistance)))

(fn ConstructionScript)

(fn UpdatePlayerList
  (params (Players :type Array%20of%20BP%20Generic%20Character%20Object%20References))
  (Variables|Default|SetPlayers Players))

(fn CalculateCameraMovement
  (Variables|Default|SetPreviousLocation (Transformation|GetWorldLocation (Variables|Default|GetSphere)))
  (bind _returnvalue (Class|GameplayStatics|GetActorArrayAverageLocation (Variables|Default|GetPlayers)))
  (Transformation|SetWorldLocation (Variables|Default|GetSphere) (Math|Vector|Lerp(Vector) (Variables|Default|GetPreviousLocation) _returnvalue (Variables|Default|GetLerpDuration)) false false))

(fn CalculateCameraDistance
  (for (_array_element _array_index) (Variables|Default|GetPlayers)
    (Utilities|IsValid _array_element
      (:Is%20Valid
        (Variables|Default|SetPlayer _array_element)
        (for _index (range (+ _array_index 1) (- (Utilities|Array|Length (Variables|Default|GetPlayers)) 1))
          (Utilities|Array|Add (Variables|Default|GetDistance) (Transformation|GetDistanceTo (Variables|Default|GetPlayer) (Utilities|Array|Get(acopy) (Variables|Default|GetPlayers) _index)))))))
  (Variables|/Script/Engine.SpringArmComponent|SetTargetArmLength (Variables|Default|GetSpringArm) (Math|Float|Clamp(Float) (.MaxValue (Math|Float|MaxOfFloatArray (Variables|Default|GetDistance))) (Variables|Default|GetMinArmLengh) (Variables|Default|GetMaxArmLengh)))
  (Utilities|Array|Clear (Variables|Default|GetDistance)))

(fn StartGame
  (Variables|Default|SetbGameStarted true))