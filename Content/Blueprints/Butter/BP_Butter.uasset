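; Butter actor that slows characters inside its box, then melts into a slippery floor.
; Box overlaps lower walk speed and restore a fixed default on exit.
; After a short delay, a timeline repeatedly multiplies the Butter component's current scale, changing height by Size and width inversely, with width clamped.
; Near-zero height spawns BP_Slippery_Floor and destroys the actor; timeline completion only destroys it.
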(event OnComponentBeginOverlap(Box)
  (params (OverlappedComponent :type Primitive%20Component%20Object%20Reference) (OtherActor :type Actor%20Object%20Reference) (OtherComp :type Primitive%20Component%20Object%20Reference) (OtherBodyIndex :type Integer) (bFromSweep :type Boolean) (SweepResult :type Hit%20Result%20Structure%20%28by%20ref%29))
  ;[1 1 1] Code caca
  (bind _ascharacter (Utilities|Casting|CastToCharacter OtherActor))
  (Variables|/Script/Engine.CharacterMovementComponent|SetMaxWalkSpeed (Variables|/Script/Engine.Character|GetCharacterMovement _ascharacter) 1.5e+02))

(event OnComponentEndOverlap(Box)
  (params (OverlappedComponent :type Primitive%20Component%20Object%20Reference) (OtherActor :type Actor%20Object%20Reference) (OtherComp :type Primitive%20Component%20Object%20Reference) (OtherBodyIndex :type Integer))
  ;[1 1 1] Code caca
  (bind _ascharacter (Utilities|Casting|CastToCharacter OtherActor))
  (Variables|/Script/Engine.CharacterMovementComponent|SetMaxWalkSpeed (Variables|/Script/Engine.Character|GetCharacterMovement _ascharacter) 6e+02))

(event EventBeginPlay
  (bind _butter (Variables|Default|GetButter))
  (bind _returnvalue (Transformation|GetRelativeTransform _butter))
  (Utilities|FlowControl|Delay 5.0)
  (bind _size (Timeline|Timeline_0 Play)
    (:Update
      (Transformation|SetRelativeTransform (Variables|Default|GetButter) (Math|Transform|MakeTransform (Transformation|GetActorLocation) "0, 0, 0" (Math|Vector|MakeVector (Math|Float|Clamp(Float) (* (- 2.0 _size) (.x (.scale _returnvalue))) 0.0 8.0) (Math|Float|Clamp(Float) (* (- 2.0 _size) (.y (.scale _returnvalue))) 0.0 7.0) (* _size (.z (.scale _returnvalue))))) false false)
      (if (<= (.z (.scale _returnvalue)) 0.001)
        (Game|SpawnActorfromClass "/Game/Blueprints/Butter/BP_Slippery_Floor.BP_Slippery_Floor_C" (Math|Transform|MakeTransform (Transformation|GetWorldLocation (Variables|Default|GetButter)) "0, 0, 0" "1.000000,1.000000,1.000000") "Undefined" "MultiplyWithRoot" 0 0)
        (Actor|DestroyActor)))
    (:Finished
      (Actor|DestroyActor))))

(fn ConstructionScript)